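; BP_EnemyChild is an enemy pawn that chases a sensed pawn and kills on contact.
; PawnSensing sighting stores the target, sets a seen flag and triggers a follow event that calls AIMoveTo toward it.
; On reaching the target, a one-shot attack guard plays a right-hand attack montage, then after a short delay loads the L_Death3 level as the death outcome.
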(event OnSeePawn(PawnSensing)
  (params (Pawn :type Pawn%20Object%20Reference))
  ;[1 1 1] Trackear
  (Variables|Default|SetPawn Pawn)
  (Variables|Default|SetVeAlPlayer true)
  (CallFunction|SeguirAlPlayer))

(event Custom|SeguirAlPlayer
  ;[1 1 1] Moverse y Matar
  (if (Variables|Default|GetVeAlPlayer)
    (AI|AIMoveTo self "0, 0, 0" (Variables|Default|GetPawn) 5.0 false
      (:OnSuccess
        (if (not (Variables|Default|GetIsAttacking))
          (Variables|Default|SetIsAttacking true)
          (Animation|Montage|PlayMontage (Variables|Character|GetMesh) "/Game/UndeadPack/Lich/Animations/Anim_Attack_Right_Montage.Anim_Attack_Right_Montage"
            (:then
              (Utilities|FlowControl|Delay 1.0)
              (Game|OpenLevel(byObjectReference) "/Game/Levels/GameOver/L_Death3.L_Death3"))))))))

(fn ConstructionScript)