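; BP_ItemBase is a collectible coin that plays a sound and increments the coin count on BP_GlobalCoinCounter when overlapped.
; Overlap sets a flag that lets Tick raise the coin each frame.
; Once its world Z reaches a fixed threshold, it disables cylinder physics, spins, turns off collision and destroys itself after a delay.
; The counter is found through GetAllActorsOfClass, using the first result.
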(event EventBeginPlay)

(event Collision|EventActorBeginOverlap
  (params (OtherActor :type Actor%20Object%20Reference))
  (CallFunction|Collected)
  (bind _output_get (Variables|Default|SetIsOverlapping true))
  ;[1 1 1] Todas las animaciones que hace la moneda al ser recogida
  (if _output_get
    (Transformation|AddActorLocalOffset "0.000000,0.000000,0.700000" false false)
    (if (<= 5e+01 (.z (Transformation|GetActorLocation)))
      (Physics|SetSimulatePhysics (Variables|Default|GetCylinder) false)
      (Transformation|AddActorLocalRotation "0.000000,30.000000,0.000000" false false)
      (bind _output_get_2 (Variables|Default|SetIsCollected true))
      (if _output_get_2
        (Collision|SetActorEnableCollision false)
        (Utilities|FlowControl|Delay 2.5)
        (Actor|DestroyActor)))))

(event EventTick
  (params (DeltaSeconds :type Float%20%28single-precision%29))
  ;[1 1 1] Todas las animaciones que hace la moneda al ser recogida
  (if (stale Collision|EventActorBeginOverlap _output_get)
    (Transformation|AddActorLocalOffset "0.000000,0.000000,0.700000" false false)
    (if (<= 5e+01 (.z (Transformation|GetActorLocation)))
      (Physics|SetSimulatePhysics (Variables|Default|GetCylinder) false)
      (Transformation|AddActorLocalRotation "0.000000,30.000000,0.000000" false false)
      (bind _output_get (Variables|Default|SetIsCollected true))
      (if _output_get
        (Collision|SetActorEnableCollision false)
        (Utilities|FlowControl|Delay 2.5)
        (Actor|DestroyActor)))))

(fn ConstructionScript)

(fn Collected
  ;[1 1 1] Al recoger una moneda reproduce un sonido e incrementa la variable GlobalCoinCounter en 1
  (Audio|PlaySound2D "/Game/Audio/CoinVanish.CoinVanish" 1.0 1.0 0.0 0 0)
  (bind _outactors (Actor|GetAllActorsOfClass "/Game/Blueprints/Actors/BP_GlobalCoinCounter.BP_GlobalCoinCounter_C"))
  (Default|IncrementCoinCount (Utilities|Array|Get(acopy) _outactors)))