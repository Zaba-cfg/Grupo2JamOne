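; Global coin counter actor that tracks collected coins and opens the way once all expected coins are picked up.
; On BeginPlay it creates the UI_Counter widget with a reference to itself and adds it to the viewport.
; IncrementCoinCount adds one to GlobalCoinCounter and, when it equals the hardcoded target of five, destroys every BP_Wall actor in the level.
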(event EventBeginPlay
  ;[1 1 1] Añade un widget con la información de las monedas recogidas
  (bind _returnvalue (UserInterface|CreateWidget "/Game/Blueprints/Widgets/UI_Counter.UI_Counter_C" 0 self))
  (bind _output_get (Variables|Default|SetCoinHUD _returnvalue))
  (UserInterface|Viewport|AddtoViewport _output_get 0))

(event Collision|EventActorBeginOverlap
  (params (OtherActor :type Actor%20Object%20Reference)))

(event EventTick
  (params (DeltaSeconds :type Float%20%28single-precision%29)))

(fn ConstructionScript)

(fn IncrementCoinCount
  ;[1 1 1] Añade 1 al contador con cada moneda recogida
  (bind _result (Math|Integer|IncrementInt (Variables|Default|GetGlobalCoinCounter))
    (:%20%20
      (bind _output_get (Variables|Default|SetGlobalCoinCounter _result))
      ;[1 1 1] Condición si se consiguen todas las monedas esperadas (5)
      (if (== 5 _output_get)
        (bind _outactors (Actor|GetAllActorsOfClass "/Game/Blueprints/BP_Wall.BP_Wall_C"))
        (Actor|DestroyActor _outactors)))))